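; Motion rule Blueprint that governs which character motions may switch into one another.
; On BeginPlay it converts MotionTable rows into per-motion switchable, forbidden and self-switch info, then passes it to InitMotionInfo with All and None IDs.
; BP wrapper functions convert E_CharacterMotion values to integer IDs for the underlying switch, end, remove and rule-update calls.
; An optional Debug flag prints switch checks and switches.
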(event `self.ReceiveBeginPlay`
  (bind ((`DataTable` _datatable)) (break `DataTableRowHandle` (`self.MotionTable`)))
  (`BlueprintMapLibrary.Map_Clear` (`self.TempMotionInfo`))
  (bind _outrownames (`DataTableFunctionLibrary.GetDataTableRowNames` _datatable))
  (for _array_element _outrownames
    (bind _returnvalue (`|GetDataTableRow` _datatable _array_element)
      (:`then`
        (bind (_type _switchablemotions _forbiddenmotions _switchself) (break `/MeleeCore/Blueprints/MotionRules/BP_MotionInfo` _returnvalue))
        (bind _returnvalue_2 (`KismetMathLibrary.Conv_ByteToInt` _type))
        (`BlueprintMapLibrary.Map_Add` (`self.TempMotionInfo`) _returnvalue_2 (make `MotionInfo` _returnvalue_2 (`self.TransEnumToIntArray` _switchablemotions) (`self.TransEnumToIntArray` _forbiddenmotions) _switchself)))))
  (`self.InitMotionInfo` (`self.TempMotionInfo`) (`KismetMathLibrary.Conv_ByteToInt` (enumliteral `/MeleeCore/Blueprints/MotionRules/E_CharacterMotion` "NewEnumerator0")) (`KismetMathLibrary.Conv_ByteToInt` (enumliteral `/MeleeCore/Blueprints/MotionRules/E_CharacterMotion` "NewEnumerator7"))))

(fn `End Motion BP`
  (params (type :type "/MeleeCore/Blueprints/MotionRules/E_CharacterMotion Enum" :default "NewEnumerator7"))
  (`MotionSwitchRule.EndMotion` (`KismetMathLibrary.Conv_ByteToInt` type)))

(fn `Is Switchable BP`
  (params (type :type "/MeleeCore/Blueprints/MotionRules/E_CharacterMotion Enum" :default "NewEnumerator7"))
  (returns (result :type "MotionCheckResult Structure"))
  (locals (resultValue :type Boolean))
  (bind _returnvalue (`MotionSwitchRule.IsSwitchable` (`KismetMathLibrary.Conv_ByteToInt` type)))
  (`|ExecutionSequence`
    (:`then_0`
      (if (`self.Debug`)
        (`KismetSystemLibrary.PrintString` (`KismetStringLibrary.Concat_StrStr` "Is Switch skill:" (`|GetEnumeratorNameAsString` type) "：" (`KismetStringLibrary.Conv_BoolToString` (`.bSwitchable` (break `MotionCheckResult` _returnvalue)))))))
    (:`then_1`
      (return _returnvalue))))

(fn `Remove Basic Rule BP`
  (params (Type :type "/MeleeCore/Blueprints/MotionRules/E_CharacterMotion Enum" :default "NewEnumerator7"))
  (`self.RemoveBasicRule` (`KismetMathLibrary.Conv_ByteToInt` Type)))

(fn `Remove Motion BP`
  (params (type :type "/MeleeCore/Blueprints/MotionRules/E_CharacterMotion Enum" :default "NewEnumerator7"))
  (`self.RemoveMotion` (`KismetMathLibrary.Conv_ByteToInt` type)))

(fn `Switch Motion BP`
  (params (type :type "/MeleeCore/Blueprints/MotionRules/E_CharacterMotion Enum" :default "NewEnumerator7"))
  (locals (Fonded :type Boolean) (SwitchableMotions :type "Array of /MeleeCore/Blueprints/MotionRules/E_CharacterMotion Enum") (ForbiddenMotions :type "Array of /MeleeCore/Blueprints/MotionRules/E_CharacterMotion Enum") (SwitchableMotionIDs :type "Array of Integer") (ForbiddenMotionIDs :type "Array of Integer"))
  (`MotionSwitchRule.SwitchMotion` (`KismetMathLibrary.Conv_ByteToInt` type))
  (if (`self.Debug`)
    (`KismetSystemLibrary.PrintString` (`KismetStringLibrary.Concat_StrStr` "Switch skill:" (`|GetEnumeratorNameAsString` type)))))

(fn `TransEnumToIntArray`
  (params (enums :type "Array of /MeleeCore/Blueprints/MotionRules/E_CharacterMotion Enum"))
  (returns (integers :type "Array of Integer"))
  (locals (Temp :type "Array of Integer"))
  (bind _temp (`local.Temp`))
  (`KismetArrayLibrary.Array_Clear` _temp)
  (for _array_element enums
    (`KismetArrayLibrary.Array_Add` _temp (`KismetMathLibrary.Conv_ByteToInt` _array_element)))
  (return (`local.Temp`)))

(fn `Update Alternative Rules BP`
  (params (rule :type "/MeleeCore/Blueprints/MotionRules/BP_MotionRuleInfo Structure (by ref)"))
  (locals (tempRules :type "Map of Integer to MotionRuleEvent Structure"))
  (bind _rules (break `/MeleeCore/Blueprints/MotionRules/BP_MotionRuleInfo` rule))
  (bind _keys (`BlueprintMapLibrary.Map_Keys` _rules))
  (for _array_element _keys
    (`BlueprintMapLibrary.Map_Add` (`local.tempRules`) (`KismetMathLibrary.Conv_ByteToInt` _array_element) (`BlueprintMapLibrary.Map_Find` _rules _array_element)))
  (`self.UpdateAlternativeRules` (`local.tempRules`)))

(fn `Update Basic Rule BP`
  (params (type :type "/MeleeCore/Blueprints/MotionRules/E_CharacterMotion Enum" :default "NewEnumerator7") (event :type "MotionRuleEvent Structure"))
  (`self.UpdateBasicRule` (`KismetMathLibrary.Conv_ByteToInt` type) (`.Callback` (break `MotionRuleEvent` event))))