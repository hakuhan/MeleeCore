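; BP_Skill manages skill lines, exposing enum-typed wrappers over name-based skill switching, execution and query functions.
; InitInfo builds the skill line list from a data table, keying each line by its type enum's string.
; Focusing a line executes the skill if that line is current, otherwise switches to it.
; When a skill ends, the line name is matched back to its enum and broadcast through OnSkillEnd.
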(event `self.InitInfo`
  (bind ((`DataTable` _datatable)) (break `DataTableRowHandle` (`self.InfoTable`)))
  (bind _outrownames (`DataTableFunctionLibrary.GetDataTableRowNames` _datatable))
  (for _array_element _outrownames
    (bind _returnvalue (`|GetDataTableRow` _datatable _array_element)
      (:`then`
        (bind (_type _switchtype _skills) (break `/MeleeCore/Blueprints/Skill/BP_SkillLineInfo` _returnvalue))
        (`KismetArrayLibrary.Array_Add` (`.SkillLines` (break `SkillTable` (`self.m_Info`))) (make `SkillLineInfo` (`|GetEnumeratorNameAsString` _type) _switchtype _skills))))))

(event `self.OnSkillEnded`
  (params (SkillLineName :type String))
  (bind _enumvalue (foreach `/MeleeCore/Blueprints/Skill/BP_SkillLineType` false)
    (:`LoopBody`
      (if (`KismetStringLibrary.EqualEqual_StrStr` (`|GetEnumeratorNameAsString` _enumvalue) SkillLineName)
        (`self.OnSkillEnd` _enumvalue)))))

(fn `Can Switch from BP`
  (params (types :type "/MeleeCore/Blueprints/Skill/BP_SkillTypes Structure") (fromAnySkill :type Boolean :default false))
  (returns (result :type Boolean))
  (locals (tempList :type "Array of String"))
  (bind _templist (`local.tempList`))
  (for _array_element (`.Types_3_ED208F2D4C3A5EF78AAD63B69A866863` (break `/MeleeCore/Blueprints/Skill/BP_SkillTypes` types))
    (`KismetArrayLibrary.Array_Add` _templist (`|GetEnumeratorNameAsString` _array_element)))
  (bind _returnvalue (`self.CanSwitchFrom` _templist fromAnySkill))
  (return _returnvalue))

(fn `Focus Skill Line BP`
  (params (type :type "/MeleeCore/Blueprints/Skill/BP_SkillLineType Enum" :default "NewEnumerator0"))
  (returns (result :type Boolean))
  (bind _result (`self.Is Current Skill BP` type))
  (if _result
    (bind _returnvalue (`self.ExecuteSkill`))
    (return _returnvalue)
    (else
      (bind _result_2 (`self.Switch Skill BP` type))
      (return _result_2))))

(fn `Is Current Skill BP`
  (params (type :type "/MeleeCore/Blueprints/Skill/BP_SkillLineType Enum" :default "NewEnumerator0"))
  (returns (result :type Boolean))
  (bind _returnvalue (`self.IsCurrentSkillLine` (`|GetEnumeratorNameAsString` type)))
  (return _returnvalue))

(fn `Switch Skill BP`
  (params (lineType :type "/MeleeCore/Blueprints/Skill/BP_SkillLineType Enum" :default "NewEnumerator0") (skillName :type String) (isForce :type Boolean))
  (returns (result :type Boolean))
  (bind _returnvalue (`self.SwitchSkill` (`|GetEnumeratorNameAsString` lineType) skillName isForce))
  (return _returnvalue))